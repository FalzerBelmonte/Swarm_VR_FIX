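; Example inventory item Blueprint for a speed potion that boosts its owner's movement when used.
; On the inventory interface's use event, it casts the item owner to Character and multiplies max walk speed and max acceleration by a fixed factor.
; It then destroys itself, with no timer or logic to revert the boost, so repeated uses compound.
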(event `/Game/BhandanaDesign/RPG_DevelopmentKit/InventorySystem/Interfaces/BPI_InventorySystem.BPI_INV_Use Item`
  (bind _ascharacter (cast `Character` (`self.ItemOwnerActor`)))
  (bind _charactermovement (`Character.CharacterMovement` _ascharacter))
  (set `CharacterMovementComponent.MaxWalkSpeed` (* (`CharacterMovementComponent.MaxWalkSpeed` _charactermovement) 1.2) _charactermovement)
  (set `CharacterMovementComponent.MaxAcceleration` (* (`CharacterMovementComponent.MaxAcceleration` _charactermovement) 1.2) _charactermovement)
  (`self.K2_DestroyActor`))

(fn `UserConstructionScript`
  (`parent.UserConstructionScript`))