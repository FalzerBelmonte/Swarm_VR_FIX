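; Swarm actor that drives many units as instances of one instanced static mesh, with a parallel brain array holding per-unit movement state.
; Tick adds units up to the set quantity, advances each along a spline with a rotating offset, then steers it toward its own point.
; A half-second timer re-picks points near the player pawn when in range, otherwise within the swarm sphere.
; Damage removes an instance overlapping the damage causer.
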(event `self.ReceiveTick`
  (params (DeltaSeconds :type "Float (single-precision)"))
  (bind _swarmunits (`self.SwarmUnits`))
  (bind _returnvalue (`InstancedStaticMeshComponent.GetInstanceCount` (`self.SwarmUnits`)))
  ;[0.05448 0.06663 0.2232] Tick: Needed to move each instance towards their individual destiniations over deltatime
  (if (< _returnvalue (`self.VAR_Quantity`))
    (`self.Add New Instance`
      (:`finished`
        _)))
  (for _index (range (+ _returnvalue 1))
    (`self.CheckSplineMovement` DeltaSeconds _index (`/Game/BhandanaDesign/Swarm_AI_Kit/Macro_Library/BPML_InstancedMeshMacros.SWARM_Get Instance Spline Progress` (`self.VAR_SwarmBrains`) _index)
      (:`SplineFinished`
        (`InstancedStaticMeshComponent.UpdateInstanceTransform` _swarmunits _index (`/Game/BhandanaDesign/Swarm_AI_Kit/Macro_Library/BPML_InstancedMeshMacros.SWARM_GetInstanceUpdatePosition` _swarmunits _index (`self.Get Target Point In Relative Space` _index) DeltaSeconds (`self.VAR_SwarmMoveSpeed`)) false (== _index _returnvalue) false)))))

(event `self.ReceiveBeginPlay`
  ;[0.05448 0.06663 0.2232] Begin Play: Currently gets local player's pawn and sets it as the target,
  ; then prepares an array of movepoints for each instance. After that, beings a custom tick for movement variation
  (`KismetSystemLibrary.Delay` 0.5)
  (bind _output_get (set `self.VAR_Target` (`Controller.K2_GetPawn` (`GameplayStatics.GetPlayerController` 0))))
  (`KismetArrayLibrary.Array_Clear` (`self.VAR_SwarmBrains`))
  (`SceneComponent.K2_SetWorldLocation` (`self.TargetMarker`) (`self.K2_GetActorLocation` _output_get) false true)
  (`self.SetActorTickEnabled` true)
  (`KismetSystemLibrary.K2_SetTimerDelegate` (delegate `CustomTick`) 0.5 true))

(event `CustomTick`
  ;[0.05448 0.06663 0.2232] Custom Tick: Assigns new points for each instance to travel t after checking which mode the instance should be traveling in
  (for _index (range (+ (`InstancedStaticMeshComponent.GetInstanceCount` (`self.SwarmUnits`)) 1))
    (`self.CheckSplineMovement` (stale `self.ReceiveTick` DeltaSeconds) _index (`/Game/BhandanaDesign/Swarm_AI_Kit/Macro_Library/BPML_InstancedMeshMacros.SWARM_Get Instance Spline Progress` (`self.VAR_SwarmBrains`) _index)
      (:`SplineFinished`
        (if (`self.Check if In Range of Target` _index)
          (`SceneComponent.K2_SetWorldLocation` (`self.TargetMarker`) (`self.K2_GetActorLocation` (`self.VAR_Target`)) false true)
          (bind (_returnvalue_x _returnvalue_y _returnvalue_z) (`KismetMathLibrary.BreakVector` (+ (`/Game/BhandanaDesign/Swarm_AI_Kit/Macro_Library/BPML_InstancedMeshMacros.SWARM_Get Instance Target Location` (`self.VAR_SwarmBrains`) _index) (* (`KismetMathLibrary.Normal` (`self.Generate Point Near Target`)) 25.0))))
          (`/Game/BhandanaDesign/Swarm_AI_Kit/Macro_Library/BPML_InstancedMeshMacros.SWARM_Set New Target Location` (`self.VAR_SwarmBrains`) _index (`KismetMathLibrary.MakeVector` (`KismetMathLibrary.FClamp` _returnvalue_x -50.0 50.0) (`KismetMathLibrary.FClamp` _returnvalue_y -50.0 50.0) (`KismetMathLibrary.FClamp` _returnvalue_z -60.0 60.0)))
          (else
            (`self.Generate Random Point in Sphere Range` _index)))))))

(event `self.ReceiveAnyDamage`
  (params (Damage :type "Float (single-precision)") (DamageType :type "DamageType Object Reference") (InstigatedBy :type "Controller Object Reference") (DamageCauser :type "Actor Object Reference"))
  (bind _returnvalue_location (`KismetMathLibrary.BreakTransform` (`self.GetTransform` DamageCauser)))
  (bind _swarmunits (`self.SwarmUnits`))
  (bind _output (`|GetArrayItem` (`InstancedStaticMeshComponent.GetInstancesOverlappingSphere` _swarmunits _returnvalue_location 1.0 true)))
  ;[1 0.125 0.125] Damage: Gets the transform of the bullet that hit the swarm, and kills the nearest instance to the impact point
  (`InstancedStaticMeshComponent.RemoveInstance` _swarmunits _output)
  (`/Engine/EditorBlueprintResources/StandardMacros.DecrementInt` (`self.VAR_Quantity`)
    (:`  `
      (`KismetArrayLibrary.Array_Remove` (`self.VAR_SwarmBrains`) _output))))

(fn `DamageGetLocation`
  (returns (Location :type "Vector Structure"))
  (return (0.0 0.0 0.0)))

(fn `UserConstructionScript`
  (bind _swarmunits (`self.SwarmUnits`))
  (bind (_returnvalue_location _returnvalue_rotation _returnvalue_scale) (`KismetMathLibrary.BreakTransform` (`SceneComponent.GetRelativeTransform` _swarmunits)))
  ;[1 1 1] Draws a sphere in editor for visual aid
  (`SphereComponent.SetSphereRadius` (`self.Sphere`) (* (`self.VAR_Quantity`) (`self.VAR_SphereSize`)) true)
  ;[1 1 1] Places the instance on the map
  (`InstancedStaticMeshComponent.AddInstance` _swarmunits (`KismetMathLibrary.MakeTransform` (0.0 0.0 0.0) (`KismetMathLibrary.RandomRotator` true) _returnvalue_scale))
  (`KismetArrayLibrary.Array_Add` (`self.VAR_SwarmBrains`) (make `/Game/BhandanaDesign/Swarm_AI_Kit/Structures/STRUCT_SwarmBrain` (0.0 0.0 0.0))))