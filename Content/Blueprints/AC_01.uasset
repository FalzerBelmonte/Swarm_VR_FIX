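; AC_01 is an actor component that spawns and updates the slot boxes of a BP_Menu_01 menu.
; SpawnMenuBox casts the owner, spawns enlarged BP_MenuBox_A actors at its MenuLocations and stores them in Locations.
; Its attach call targets the menu itself, not the new box.
; SetSlot forwards a Section and Value to every stored box through SetValue.
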(event `SetSlot`
  (params (Section :type "/Game/Blueprints/enums/EN_MenuSections Enum" :default "NewEnumerator0") (Value :type "Float (double-precision)"))
  (for _array_element (`self.Locations`)
    (`/Game/Blueprints/bps/BP_MenuBox_A.SetValue` _array_element Section Value)))

(event `SpawnMenuBox`
  (params (`Number of Slot` :type Integer :default 1))
  (bind _asbp_menu_01 (cast `/Game/Blueprints/bps/BP_Menu_01` (`self.GetOwner`)))
  (for _index (range (+ `Number of Slot` 1))
    (bind _output (`|GetArrayItem` (`/Game/Blueprints/bps/BP_Menu_01.MenuLocations` _asbp_menu_01) _index))
    (bind _returnvalue (`|SpawnActorFromClass` "/Game/Blueprints/bps/BP_MenuBox_A.BP_MenuBox_A_C" (`KismetMathLibrary.MakeTransform` (`SceneComponent.K2_GetComponentLocation` _output) (struct) (2.0 2.0 2.0)) "Undefined" "OverrideRootScale" _asbp_menu_01 true 0 "" "" 0.0 "NewEnumerator7" 1.0 20.0 null))
    (`KismetArrayLibrary.Array_Set` (`self.Locations`) _index _returnvalue true)
    (`Actor.K2_AttachToComponent` _asbp_menu_01 _output "None" "KeepWorld" "KeepWorld" "KeepWorld" true)))

(event `self.ReceiveBeginPlay`)