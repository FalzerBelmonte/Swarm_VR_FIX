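; Bullet director actor that fires BP_Bullet_02 projectiles at the left and right enemies while active and outside the menu.
; Tick throttles firing with a Delay scaled by DeltaSeconds and RPS, then checks each controller's pressed state to spawn bullets with side, target and speed.
; BeginPlay caches the WD_info widget, seeds its float and activates firing.
; ReportController exposes both press states, while ReportValue returns only constant zeros.
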(event `self.ReceiveBeginPlay`
  (bind _aswd_info (cast `/Game/Blueprints/WD_info` (`WidgetComponent.GetUserWidgetObject` (`self.Widget`))))
  (bind _output_get (set `self.info` _aswd_info))
  (set `/Game/Blueprints/WD_info.infoFloat` 444.0 _output_get)
  (set `self.Active` true))

(event `self.ReceiveTick`
  (params (DeltaSeconds :type "Float (single-precision)"))
  (bind _bulletspeed (`self.BulletSpeed`))
  (bind _spawnerlocation (`self.SpawnerLocation`))
  (`KismetSystemLibrary.Delay` (* DeltaSeconds (`self.RPS`)))
  (if (and (`self.Active`) (not (`self.inMenu`)))
    (`|ExecutionSequence`
      (:`then_0`
        (switch `/Game/Blueprints/enums/EN_ControllerLeft` (`self.CNTLeft`)
          (:`NewEnumerator0`
            (`|SpawnActorFromClass` "/Game/Blueprints/bps/BP_Bullet_02.BP_Bullet_02_C" (`KismetMathLibrary.MakeTransform` (0.0 -3000.0 10.0)) "Undefined" "OverrideRootScale" null _spawnerlocation (`self.EnemyLeft`) 0 (`self.Left`) _bulletspeed null))))
      (:`then_1`
        (switch `/Game/Blueprints/enums/EN_ControllerRight` (`self.CNTRight`)
          (:`NewEnumerator0`
            (`|SpawnActorFromClass` "/Game/Blueprints/bps/BP_Bullet_02.BP_Bullet_02_C" (`KismetMathLibrary.MakeTransform` (0.0 -3000.0 10.0)) "Undefined" "OverrideRootScale" null _spawnerlocation (`self.EnemyRight`) 0 (`self.Right`) _bulletspeed null)))))))

(fn `ReportController`
  (returns (Left :type "/Game/Blueprints/enums/EN_ControllerLeft Enum") (Right :type "/Game/Blueprints/enums/EN_ControllerRight Enum"))
  (return "NewEnumerator0" "NewEnumerator0"))

(fn `ReportValue`
  (returns (Value :type "Float (double-precision)") (ID :type Integer))
  (return 0.0 0))

(fn `UserConstructionScript`)