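; Projectile actor that, once activated, teleport-steps each tick toward a point projected past its target and destroys itself on arrival.
; Awake positions and aims it, optionally firing after a delay, and stretches the Head collision to per-frame travel distance.
; Type A Head and Back overlaps send default or random damage through BPI_DMGEnemy, then destroy it.
; Blast line-traces through the spawner location to report the bullet's position before destroying it.
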(event `self.ReceiveBeginPlay`
  (set `self.TransfromRefrence` (`SceneComponent.GetRelativeTransform` (`self.Head`)))
  (`self.MakeCollisionSize` (`self.Speed`) (`self.Target`)))

(event `self.ReceiveTick`
  (params (DeltaSeconds :type "Float (single-precision)"))
  (if (`self.Active`)
    (bind _targetmeet (`self.Move` (`self.TargetPlus`) (`self.Speed`) DeltaSeconds))
    (if _targetmeet
      (`self.BulletDestroy`))))

(event `Debug_ShowDirections`
  (bind _returnvalue (`self.K2_GetActorLocation`))
  (bind _target (`self.Target`))
  (bind _output_get (set `self.TargetPlus` (+ _returnvalue (* (`KismetMathLibrary.GetForwardVector` (`KismetMathLibrary.FindLookAtRotation` _returnvalue _target)) (`KismetMathLibrary.FTrunc` (* (`KismetMathLibrary.Vector_Distance` _returnvalue _target) (`self.PlusDistance`)))))))
  (`KismetSystemLibrary.LineTraceSingle` :`Start` _returnvalue :`End` _output_get :`TraceChannel` "TraceTypeQuery1" :`DrawDebugType` "ForDuration" :`TraceColor` (struct :`R` 0.08439 :`G` 0.069942 :`B` 0.166667 :`A` 1.0) :`TraceHitColor` (struct :`R` 0.485203 :`G` 0.010197 :`B` 1.0 :`A` 1.0) :`DrawTime` 80.0)
  (`self.MakeCollisionSize` (`self.Speed`) (`self.Target`)))

(event `Fire`
  (set `self.Active` true))

(event `Awake`
  (params (Location :type "Vector Structure") (Time :type "Float (double-precision)") (Fire :type Boolean))
  (bind _returnvalue (`self.K2_GetActorLocation`))
  (bind _target (`self.Target`))
  (`|ExecutionSequence`
    (:`then_0`
      (`self.K2_SetActorLocation` Location)
      (`self.K2_SetActorRotation` (`KismetMathLibrary.FindLookAtRotation` Location (`self.Target`)))
      (`self.MakeCollisionSize` (`self.Speed`) (`self.Target`))
      (set `self.TargetPlus` (+ _returnvalue (* (`KismetMathLibrary.GetForwardVector` (`KismetMathLibrary.FindLookAtRotation` _returnvalue _target)) (`KismetMathLibrary.FTrunc` (* (`KismetMathLibrary.Vector_Distance` _returnvalue _target) (`self.PlusDistance`)))))))
    (:`then_1`
      (if Fire
        (`KismetSystemLibrary.Delay` Time)
        (`self.Fire`)))))

(event `BulletDestroy`
  (`self.K2_DestroyActor`))

(event `Blast`
  (`self.BlastSetup`)
  (set `self.Active` false)
  (`self.BulletDestroy`))

(event `self.Head.OnComponentBeginOverlap`
  (params (OverlappedComponent :type "PrimitiveComponent Object Reference") (OtherActor :type "Actor Object Reference") (OtherComp :type "PrimitiveComponent Object Reference") (OtherBodyIndex :type Integer) (bFromSweep :type Boolean) (SweepResult :type "HitResult Structure (by ref)"))
  (if (`KismetSystemLibrary.DoesImplementInterface` OtherActor "/Game/Blueprints/BPI_DMGEnemy.BPI_DMGEnemy_C")
    (switch `/Game/Blueprints/EN_WeaponType` (`self.WeaponType`)
      (:`NewEnumerator0`
        (message `/Game/Blueprints/BPI_DMGEnemy.DamageDefault` OtherActor)
        (`self.BulletDestroy` :!label _label)))))

(event `self.Back.OnComponentBeginOverlap`
  (params (OverlappedComponent :type "PrimitiveComponent Object Reference") (OtherActor :type "Actor Object Reference") (OtherComp :type "PrimitiveComponent Object Reference") (OtherBodyIndex :type Integer) (bFromSweep :type Boolean) (SweepResult :type "HitResult Structure (by ref)"))
  (if (`KismetSystemLibrary.DoesImplementInterface` OtherActor "/Game/Blueprints/BPI_DMGEnemy.BPI_DMGEnemy_C")
    (switch `/Game/Blueprints/EN_WeaponType` (`self.WeaponType`)
      (:`NewEnumerator0`
        (message `/Game/Blueprints/BPI_DMGEnemy.DamageValue` OtherActor (`KismetMathLibrary.RandomFloatInRange` 0.0 20.0))
        (goto _label)))))

(event `MakeCollisionSize`
  (params (Speed :type "Float (double-precision)") (Target :type "Vector Structure"))
  (bind _transfromrefrence (`self.TransfromRefrence`))
  (bind _returnvalue_x (`KismetMathLibrary.BreakVector` (`KismetMathLibrary.GetDirectionUnitVector` (`self.K2_GetActorLocation`) Target)))
  (bind _returnvalue (* Speed (`GameplayStatics.GetWorldDeltaSeconds`)))
  (`SceneComponent.K2_SetRelativeTransform` (`self.Head`) (`KismetMathLibrary.MakeTransform` (`KismetMathLibrary.MakeVector` (+ (/ (* _returnvalue_x _returnvalue) 2.0) (.x (.location _transfromrefrence))) (.y (.location _transfromrefrence)) (.z (.location _transfromrefrence))) (.rotation _transfromrefrence) (`KismetMathLibrary.MakeVector` (/ _returnvalue 60.0) (.y (.scale _transfromrefrence)) (.z (.scale _transfromrefrence)))) false false)
  (`KismetSystemLibrary.PrintString` (`KismetStringLibrary.Concat_StrStr` (`KismetStringLibrary.Conv_DoubleToString` _returnvalue) " \n xxxx " "" " \n -     ") true true (struct :`R` 1.0 :`G` 0.568663 :`B` 0.281854 :`A` 1.0) 20.0))

(fn `BlastSetup`
  (bind _spawnerlocation (`self.SpawnerLocation`))
  (bind _returnvalue (+ _spawnerlocation (0.0 0.0 -200.0)))
  (bind (_outhit _returnvalue_2) (`KismetSystemLibrary.LineTraceSingleForObjects` :`Start` _returnvalue :`End` (+ _returnvalue (* (`KismetMathLibrary.GetForwardVector` (`KismetMathLibrary.FindLookAtRotation` _returnvalue _spawnerlocation)) (`KismetMathLibrary.FTrunc` (* (`KismetMathLibrary.Vector_Distance` _returnvalue _spawnerlocation) 10000.0)))) :`ObjectTypes` (`|MakeArray` (enumliteral `EObjectTypeQuery` "ObjectTypeQuery2")) :`DrawDebugType` "ForDuration"))
  (if _returnvalue_2
    (message `/Game/Blueprints/BPI_Report.ReportLocation` (`.HitActor` (`GameplayStatics.BreakHitResult` _outhit)) true (`self.ID`) (`self.K2_GetActorLocation`))
    (return)))

(fn `Move`
  (params (Target :type "Vector Structure") (Speed :type "Float (double-precision)" :default 120.0) (DS :type "Float (double-precision)"))
  (returns (TargetMeet :type Boolean))
  (bind _returnvalue (`self.K2_GetActorLocation`))
  (bind _returnvalue_2 (* Speed DS))
  (bind _returnvalue_3 (+ (* (`KismetMathLibrary.GetDirectionUnitVector` _returnvalue Target) _returnvalue_2) _returnvalue))
  (`self.K2_SetActorRotation` (`KismetMathLibrary.FindLookAtRotation` _returnvalue Target))
  (if (> (`KismetMathLibrary.Vector_Distance` Target _returnvalue_3) _returnvalue_2)
    (`self.K2_SetActorLocation` _returnvalue_3)
    (return false)
    (else
      (`self.K2_SetActorLocation` Target)
      (return true))))

(fn `UserConstructionScript`)