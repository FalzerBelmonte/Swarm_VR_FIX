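; Bullet Blueprint that damages actors implementing BPI_DMGEnemy on overlap, then destroys itself.
; On BeginPlay it resizes the Head collision from its relative transform and the frame delta time, then fires.
; For weapon Type A, a Head overlap sends a default damage message and a Back overlap sends a random damage value.
; Both paths then apply a fixed base damage.
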(event `self.ReceiveBeginPlay`
  (bind _head (`self.Head`))
  (bind _returnvalue (`self.MakeCollisionSize` (`SceneComponent.GetRelativeTransform` _head) (`GameplayStatics.GetWorldDeltaSeconds`)))
  (`SceneComponent.K2_SetRelativeTransform` _head _returnvalue false false)
  (`self.Fire`))

(event `self.Head.OnComponentBeginOverlap`
  (params (OverlappedComponent :type "PrimitiveComponent Object Reference") (OtherActor :type "Actor Object Reference") (OtherComp :type "PrimitiveComponent Object Reference") (OtherBodyIndex :type Integer) (bFromSweep :type Boolean) (SweepResult :type "HitResult Structure (by ref)"))
  (if (`KismetSystemLibrary.DoesImplementInterface` OtherActor "/Game/Blueprints/BPI_DMGEnemy.BPI_DMGEnemy_C")
    (switch `/Game/Blueprints/EN_WeaponType` (`self.WeaponType`)
      (:`NewEnumerator0`
        (message `/Game/Blueprints/BPI_DMGEnemy.DamageDefault` OtherActor)
        (`GameplayStatics.ApplyDamage` (stale `self.Back.OnComponentBeginOverlap` OtherActor) 1.0 null self "/Script/Engine.DamageType" :!label _label)
        (`self.DestroyBullet`)))))

(event `self.Back.OnComponentBeginOverlap`
  (params (OverlappedComponent :type "PrimitiveComponent Object Reference") (OtherActor :type "Actor Object Reference") (OtherComp :type "PrimitiveComponent Object Reference") (OtherBodyIndex :type Integer) (bFromSweep :type Boolean) (SweepResult :type "HitResult Structure (by ref)"))
  (if (`KismetSystemLibrary.DoesImplementInterface` OtherActor "/Game/Blueprints/BPI_DMGEnemy.BPI_DMGEnemy_C")
    (switch `/Game/Blueprints/EN_WeaponType` (`self.WeaponType`)
      (:`NewEnumerator0`
        (message `/Game/Blueprints/BPI_DMGEnemy.DamageValue` OtherActor (`KismetMathLibrary.RandomFloatInRange` 0.0 20.0))
        (goto _label)))))

(fn `UserConstructionScript`)