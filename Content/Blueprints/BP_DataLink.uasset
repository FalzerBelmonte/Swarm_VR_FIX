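; BP_DataLink is a relay actor that passes enemy state events to other objects.
; Pause, begin, alive and dead events re-broadcast the enemy ID through Call dispatchers, with alive and dead ignoring negative IDs.
; On BeginPlay it moves to a hardcoded transform, and ReportController returns left and right controller references.
; The type and location report events are empty, and ReportValue returns only zeros.
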(event `self.ReceiveBeginPlay`
  (`|ExecutionSequence`
    (:`then_1`
      (`self.K2_SetActorTransform` (`KismetMathLibrary.MakeTransform` (1200.0 1500.0 200.0) (`KismetMathLibrary.FindLookAtRotation` (`self.K2_GetActorLocation`) (0.0 0.0 160.0)))))))

(event `EnemyPause`
  (params (EnemyID :type Integer) (Pause :type Boolean))
  (`self.SwitchEnemyPause` Pause EnemyID))

(event `EnemyBegin`
  (params (EnemyID :type Integer))
  (`self.SwitchEnemyBegin` EnemyID))

(event `SetEnemyAlive`
  (params (EnemyID :type Integer))
  (if (> EnemyID -1)
    (`self.EnemyAlive` EnemyID)))

(event `/Game/Blueprints/BPI_Report.ReportDead`
  (params (EnemyID :type Integer))
  (if (> EnemyID -1)
    (`self.EnemyDead` EnemyID)))

(event `/Game/Blueprints/BPI_Report.ReportTypeA`
  (params (Value :type "Float (single-precision)") (ID :type Integer)))

(event `/Game/Blueprints/BPI_Report.ReportTypeB`
  (params (Spawn :type Boolean) (Damage :type "Float (single-precision)") (ID :type Integer) (LocationA :type "Vector Structure") (LocationB :type "Vector Structure") (WeaponType :type "/Game/Blueprints/enums/EN_WeaponType Enum" :default "NewEnumerator0")))

(event `/Game/Blueprints/BPI_Report.ReportLocation`
  (params (Bullet :type Boolean) (ID :type Integer) (Location :type "Vector Structure")))

(fn `ReportController`
  (returns (Left :type "/Game/Blueprints/enums/EN_ControllerLeft Enum") (Right :type "/Game/Blueprints/enums/EN_ControllerRight Enum"))
  (return (`self.ControllerLeft`) (`self.ControllerRight`)))

(fn `ReportValue`
  (returns (Value :type "Float (double-precision)") (ID :type Integer))
  (return 0.0 0))

(fn `UserConstructionScript`)