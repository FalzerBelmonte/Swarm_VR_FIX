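; Enemy spawner for a VR game that creates a population of BP_Enemy_A units once and reuses them in waves.
; Tick drives staggered, randomly delayed spawns, stacking units by height and assigning target locations round-robin.
; DataLink death and alive events update the Dead array, with deaths also lowering GameState score and counting kills.
; When kills reach Population, the pooled units are reawakened one by one unless the game is paused.
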(event `self.ReceiveBeginPlay`
  (bind _datalink (`self.DataLink`))
  (if (`self.Active`)
    (set `self.Active` false)
    (`|ExecutionSequence`
      (:`then_0`
        (bind _asgame_state_vr (cast `/Game/Blueprints/GameStateVR` (`GameplayStatics.GetGameState`))
          (:`then`
            (set `self.GameState` _asgame_state_vr)
            (add `/Game/Blueprints/BP_DataLink.EnemyDead` _datalink (delegate `EnemyDead`))
            (add `/Game/Blueprints/BP_DataLink.EnemyAlive` _datalink (delegate `EnemyAlive`)))
          (:`CastFailed`
            (`KismetSystemLibrary.PrintString` ">>> GameState missing" true true (struct :`R` 0.994792 :`G` 1.0 :`B` 0.989583 :`A` 1.0) 80.0))))
      (:`then_1`
        (set `self.Active` true)))))

(event `EnemyDead`
  (params (EnemyID :type Integer))
  (`KismetArrayLibrary.Array_Set` (`self.Dead`) EnemyID true true)
  (`/Game/Blueprints/GameStateVR.Score_Change` (`self.GameState`) EnemyID -1)
  (`/Engine/EditorBlueprintResources/StandardMacros.IncrementInt` (`self.temp_EnemyDestroyd`)))

(event `EnemyAlive`
  (params (EnemyID :type Integer))
  (`KismetArrayLibrary.Array_Set` (`self.Dead`) EnemyID false true))

(event `FirstSpawn`
  (`KismetSystemLibrary.Delay` (`KismetMathLibrary.RandomFloatInRange` 0.18 0.22))
  (bind (_returnvalue _enemyid) (`self.SpawnEnemyCPP` (`self.temp_EnemyCounter`) (`KismetStringLibrary.Conv_NameToString` "TU-5RC")))
  (`KismetArrayLibrary.Array_Set` (`self.EnemyUnitsCPP`) _enemyid _returnvalue true)
  (`/Game/Blueprints/GameStateVR.Score_Change` (`self.GameState`) _enemyid 1)
  (set `self.SpawnFirst` (< (`self.temp_EnemyCounter`) (`self.Population`)))
  (`/Engine/EditorBlueprintResources/StandardMacros.IncrementInt` (`self.temp_EnemyCounter`)))

(event `self.ReceiveTick`
  (params (DeltaSeconds :type "Float (single-precision)"))
  (if (`self.Active`)
    (`|ExecutionSequence`
      (:`then_0`
        (if (`self.SpawnFirst`)
          (`self.FirstSpawn`)))
      (:`then_1`
        (if (`self.RestartEnemy`)
          (`self.EnemyRestart`)))
      (:`then_2`
        (`KismetSystemLibrary.Delay` 2.4)
        (`self.RefreshPopulation`)))))

(event `RefreshPopulation`
  (if (>= (`self.temp_EnemyDestroyd`) (`self.Population`))
    (bind _output_get (set `self.temp_EnemyCounter` 0))
    (set `self.temp_EnemyDestroyd` _output_get)
    (set `self.RestartEnemy` true)))

(event `EnemyRestart`
  (bind _temp_enemycounter (`self.temp_EnemyCounter`))
  (`KismetSystemLibrary.Delay` (`KismetMathLibrary.RandomFloatInRange` 0.18 0.3))
  (if (not (`/Game/Blueprints/GameStateVR.GamePause` (`self.GameState`)))
    (`/Game/Blueprints/BP_DataLink.SetEnemyAlive` (`self.DataLink`) _temp_enemycounter)
    (`/Game/Blueprints/GameStateVR.Score_Change` (`self.GameState`) _temp_enemycounter 1)
    (`EN_A.Awake` (`|GetArrayItem` (`self.EnemyUnitsCPP`) _temp_enemycounter) false false 60.0 (`self.Speed`) 8 0.75 360.0 30.0)
    (set `self.RestartEnemy` (< (`self.temp_EnemyCounter`) (`self.Population`)))
    (`/Engine/EditorBlueprintResources/StandardMacros.IncrementInt` (`self.temp_EnemyCounter`))))

(fn `ReportController`
  (returns (Left :type "/Game/Blueprints/EN_ControllerLeft Enum") (Right :type "/Game/Blueprints/EN_ControllerRight Enum"))
  (return "NewEnumerator0" "NewEnumerator0"))

(fn `ReportValue`
  (returns (Value :type "Float (double-precision)") (ID :type Integer))
  (return 0.0 0))

(fn `SpawnEnemyCPP`
  (params (index :type Integer) (EnemyName :type String))
  (returns (ReturnValue :type "/Game/Blueprints/BP_Enemy_A Object Reference") (EnemyID :type Integer))
  (set `self.EnemySpawnGate` (mod index (`KismetArrayLibrary.Array_Length` (`self.TargetLocations`))))
  (bind _returnvalue (`|SpawnActorFromClass` "/Game/Blueprints/BP_Enemy_A.BP_Enemy_A_C" (`KismetMathLibrary.MakeTransform` (`KismetMathLibrary.MakeVector` 0.0 0.0 (`KismetMathLibrary.Conv_IntToDouble` (+ (* index 200) 1400))) (struct) (4.0 4.0 4.0)) "Undefined" "OverrideRootScale" null (`self.DataLink`) "NewEnumerator3" "NewEnumerator0" index (`KismetStringLibrary.Conv_StringToName` (`KismetStringLibrary.Concat_StrStr` EnemyName (`KismetTextLibrary.Conv_TextToString` (`KismetTextLibrary.Conv_Int64ToText` (`KismetMathLibrary.RandomInteger64InRange` 0 87432))))) (`|GetArrayItem` (`self.TargetLocations`) (`self.EnemySpawnGate`)) (`self.StartLocation`) null))
  (`EN_A.Awake` _returnvalue false true 60.0 (`self.Speed`) 8 0.75 360.0 30.0)
  (return _returnvalue index))

(fn `UserConstructionScript`)