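; BP_Enemy_01 is an enemy Blueprint that shows its health through a widget component.
; On BeginPlay it casts the widget to WD_info, stores it and passes Health into its InfoFloat, then appends a random number to EnemyName.
; DamageGetLocation returns the actor's location.
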(event `self.ReceiveBeginPlay`
  (bind _aswd_info (cast `/Game/Blueprints/WD_info` (`WidgetComponent.GetUserWidgetObject` (`self.Widget`))))
  (set `self.infoTXT` _aswd_info)
  (set `/Game/Blueprints/WD_info.infoFloat` (`self.Health`) (`self.infoTXT`))
  (set `self.EnemyName` (`KismetStringLibrary.Conv_StringToName` (`KismetStringLibrary.Concat_StrStr` (`KismetStringLibrary.Conv_NameToString` (`self.EnemyName`)) (`KismetTextLibrary.Conv_TextToString` (`KismetTextLibrary.Conv_Int64ToText` (`KismetMathLibrary.RandomInteger64InRange` 0 87432)))))))

(fn `DamageGetLocation`
  (returns (Location :type "Vector Structure"))
  (return (`self.K2_GetActorLocation`)))

(fn `UserConstructionScript`)