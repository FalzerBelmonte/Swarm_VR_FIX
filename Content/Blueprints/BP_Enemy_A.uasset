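; BP_Enemy_A is an enemy actor that takes damage and displays its ID and health on text renders.
; On BeginPlay it registers with DataLink, binds begin and pause callbacks, caches bullet damage and activates itself.
; While active, default or supplied damage is randomised to 80–100% before the health check.
; Death or reaching path end reports to DataLink and destroys the enemy; the begin handler and DamageGetLocation are stubs.
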(event `SwitchEnemyPause`
  (params (Pause :type Boolean) (EnemyID :type Integer))
  (`self.PauseEnemy` Pause))

(event `SwitchEnemyBegin`
  (params (EnemyID :type Integer)))

(event `self.ReceiveBeginPlay`
  (bind _datalink (`self.DataLink`))
  (`|ExecutionSequence`
    (:`then_0`
      (if (`KismetSystemLibrary.IsValid` _datalink)
        (`/Game/Blueprints/BP_DataLink.SetEnemyAlive` _datalink (`self.EnemyID`))
        (add `/Game/Blueprints/BP_DataLink.SwitchEnemyBegin` _datalink (delegate `SwitchEnemyBegin`))
        (add `/Game/Blueprints/BP_DataLink.SwitchEnemyPause` _datalink (delegate `SwitchEnemyPause`))
        (set `self.BulletDamage` (`/Game/Blueprints/BP_DataLink.BulletDamage` _datalink))))
    (:`then_1`
      (`TextRenderComponent.K2_SetText` (`self.TextRender1`) (`KismetTextLibrary.Conv_StringToText` (`KismetStringLibrary.Conv_IntToString` (`self.EnemyID`))))
      (`TextRenderComponent.K2_SetText` (`self.TextRender`) (`KismetTextLibrary.Conv_StringToText` (`KismetStringLibrary.Conv_DoubleToString` (`self.GetHealth`))))
      (`self.ActivateEnemy`))))

(event `/Game/Blueprints/BPI_DMGEnemy.DamageDefault`
  (bind _bulletdamage (`self.BulletDamage`))
  (if (`self.Active`)
    (bind _returnvalue (`self.CheckHealth` (`KismetMathLibrary.RandomFloatInRange` (* _bulletdamage 0.8) _bulletdamage)))
    (`TextRenderComponent.K2_SetText` (`self.TextRender`) (`KismetTextLibrary.Conv_StringToText` (`KismetStringLibrary.Conv_DoubleToString` (`self.GetHealth`))))
    (if _returnvalue
      (message `/Game/Blueprints/BPI_Report.ReportDead` (`self.DataLink`) (`self.EnemyID`) :!label _label)
      (`self.DestroyEnemy`)
      (`TextRenderComponent.K2_SetText` (`self.TextRender`) (`KismetTextLibrary.Conv_StringToText` (`KismetStringLibrary.Conv_DoubleToString` 100.0))))))

(event `/Game/Blueprints/BPI_DMGEnemy.DamageValue`
  (params (Damage :type "Float (single-precision)"))
  (if (`self.Active`)
    (bind _returnvalue (`self.CheckHealth` (`KismetMathLibrary.RandomFloatInRange` (* Damage 0.8) Damage)))
    (`TextRenderComponent.K2_SetText` (`self.TextRender`) (`KismetTextLibrary.Conv_StringToText` (`KismetStringLibrary.Conv_DoubleToString` (`self.GetHealth`))))
    (if _returnvalue
      (goto _label))))

(event `self.EndPath`
  (message `/Game/Blueprints/BPI_Report.ReportDead` (`self.DataLink`) (`self.EnemyID`))
  (`self.DestroyEnemy`)
  (`TextRenderComponent.K2_SetText` (`self.TextRender`) (`KismetTextLibrary.Conv_StringToText` (`KismetStringLibrary.Conv_DoubleToString` 100.0))))

(fn `DamageGetLocation`
  (returns (Location :type "Vector Structure"))
  (return (0.0 0.0 0.0)))

(fn `UserConstructionScript`)