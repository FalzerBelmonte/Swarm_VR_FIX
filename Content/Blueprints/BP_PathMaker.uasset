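; BP_PathMaker is an actor that visualizes a looping path as debug points drawn relative to its location.
; Each Tick it accumulates delta time, wrapping past Max, samples the Path vector curve at that time, scales the result and offsets it by the actor location.
; Short-lived red points form a trail, while disconnected nodes for moving a Cone along the path and drawing debug boxes never run.
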(event `self.ReceiveTick`
  (params (DeltaSeconds :type "Float (single-precision)"))
  (bind _output_get (set `self.temp_01` (+ DeltaSeconds (`self.temp_01`))))
  (if (> _output_get (`self.Max`))
    (set `self.temp_01` (- (`self.temp_01`) (`self.Max`))))
  (`KismetSystemLibrary.DrawDebugPoint` (+ (* (`CurveVector.GetVectorValue` (`self.Path`) (`self.temp_01`)) (`self.Scale`)) (`self.K2_GetActorLocation`)) 2.0 (struct :`R` 1.0 :`B` 0.109999 :`A` 1.0) 10.0))

(fn `UserConstructionScript`)