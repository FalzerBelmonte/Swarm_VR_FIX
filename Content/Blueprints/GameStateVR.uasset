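; VR game state that coordinates players, scoreboards and enemy waves through a shared BP_DataLink actor.
; On introMap, BeginPlay spawns the DataLink, hands it to VR pawns and builds scoreboards at name-matched TargetPoints.
; Events register and set up ready players, route score changes to boards and relay enemy pause.
; SpawnEnemyUnits feeds target locations and DataLink to a new spawner, but its only call here is unreachable.
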(event `PlayerReady`
  (params (ID :type Integer))
  (`KismetArrayLibrary.Array_Set` (`self.Players`) ID 100 true)
  (if true
    (for _array_element (`self.PlayerArray`)
      (if (== ID (`PlayerState.PlayerId` _array_element))
        (bind _asvr_pawn (cast `/Game/Blueprints/VR_Pawn` (`PlayerState.PawnPrivate` _array_element)))
        (set `/Game/Blueprints/VR_Pawn.DataLink` (`self.DataLink`) _asvr_pawn)
        (`KismetSystemLibrary.Delay` 0.1)
        (`/Game/Blueprints/VR_Pawn.SetupPlayer` _asvr_pawn ID)))))

(event `self.ReceiveBeginPlay`
  (bind _returnvalue (`GameplayStatics.GetCurrentLevelName` true))
  (if (`KismetStringLibrary.EqualEqual_StrStr` _returnvalue "introMap")
    (`|ExecutionSequence`
      (:`then_0`
        (bind _returnvalue_2 (`|SpawnActorFromClass` "/Game/Blueprints/BP_DataLink.BP_DataLink_C" (`KismetMathLibrary.MakeTransform` (0.0 0.0 200.0)) "Undefined" "OverrideRootScale" null null))
        (set `self.DataLink` _returnvalue_2)
        (for _array_element (`self.PlayerArray`)
          (if (`KismetSystemLibrary.IsValid` _array_element)
            (bind _asvr_pawn (cast `/Game/Blueprints/VR_Pawn` (`PlayerState.PawnPrivate` _array_element)))
            (set `/Game/Blueprints/VR_Pawn.DataLink` (`self.DataLink`) _asvr_pawn))))
      (:`then_1`
        (`self.SetTargetScore`)))))

(event `EnemyPause`
  (params (Pause :type Boolean))
  (`/Game/Blueprints/BP_DataLink.EnemyPause` (`self.DataLink`) 0 Pause)
  (set `self.GamePause` Pause))

(event `Score_Change`
  (params (ID :type Integer) (Value :type Integer))
  (bind _returnvalue (mod ID 3))
  (message `/Game/Blueprints/BPI_Report.ReportTypeA` (`|GetArrayItem` (`self.ScoreBoard`) _returnvalue) (`KismetMathLibrary.Conv_IntToDouble` Value) _returnvalue))

(event `SpawnEnemyUnits`
  (`KismetSystemLibrary.Delay` 0.05)
  (bind _returnvalue (`|SpawnActorFromClass` "/Game/Blueprints/BP_EnemySpawner.BP_EnemySpawner_C" (`KismetMathLibrary.MakeTransform` (`self.SpawnerLocation`) (struct :`Yaw` 180.0) (5.0 5.0 5.0)) "Undefined" "OverrideRootScale" null false true false 180.0 (`self.TargetLocations`) (0.0 0.0 3200.0) 31 (`self.Wave`) (`self.DataLink`) null))
  (set `self.EnemySpawner` _returnvalue)
  (`KismetSystemLibrary.PrintString` "------------------------------" true true (struct :`R` 1.0 :`G` 0.716873 :`A` 1.0)))

(fn `SetTargetScore`
  (bind _targetlocations (`self.TargetLocations`))
  (bind _outactors (`GameplayStatics.GetAllActorsOfClass` "/Script/Engine.TargetPoint"))
  (bind _output_get (set `self.Targets` _outactors))
  (for _array_element _output_get
    (switch `string` (`KismetSystemLibrary.GetDisplayName` _array_element)
      (:`TargetA`
        (bind _returnvalue (`self.K2_GetActorLocation` _array_element))
        (`KismetArrayLibrary.Array_Set` _targetlocations 0 _returnvalue true))
      (:`TargetB`
        (`KismetArrayLibrary.Array_Set` _targetlocations 1 _returnvalue true))
      (:`TargetC`
        (`KismetArrayLibrary.Array_Set` _targetlocations 2 _returnvalue true))))
  (for (_array_element_2 _array_index) (`self.TargetLocations`)
    (bind _returnvalue_2 (`|SpawnActorFromClass` "/Game/Blueprints/bps/BP_ScoreBoard.BP_ScoreBoard_C" (`KismetMathLibrary.MakeTransform` _array_element_2 (`KismetMathLibrary.FindLookAtRotation` _array_element_2 (0.0 0.0 0.0)) (4.0 4.0 4.0)) "Undefined" "OverrideRootScale" null _array_index null))
    (`KismetArrayLibrary.Array_Set` (`self.ScoreBoard`) _array_index _returnvalue_2 true))
  (return))

(fn `UserConstructionScript`)