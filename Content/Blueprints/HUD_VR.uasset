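; HUD_VR manages the world-space VR menus on introMap for starting or resuming play and quitting.
; After a short delay it spawns a BP_Menu_01 along each GameStateVR target direction, showing or hiding them by moving their height.
; MenuReport takes either controller's press: Play and Resume unpause enemies and hide menus, with Play relabeled Resume.
; A DoOnce limits Value 01 changes to one per press; GetMenuData and enemy spawning are unwired.
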(event `self.ReceiveBeginPlay`
  (bind _returnvalue (`GameplayStatics.GetCurrentLevelName` true))
  (if (`KismetStringLibrary.EqualEqual_StrStr` _returnvalue "introMap")
    (bind _asgame_state_vr (cast `/Game/Blueprints/GameStateVR` (`GameplayStatics.GetGameState`))
      (:`then`
        (set `self.GameState` _asgame_state_vr)
        (`KismetSystemLibrary.Delay` 0.2)
        (`self.Add Menus`))
      (:`CastFailed`
        (`KismetSystemLibrary.PrintString` ">>> GameState missing" true true (struct :`R` 0.994792 :`G` 1.0 :`B` 0.989583 :`A` 1.0) 80.0)))))

(event `Add Menus`
  (for (_array_element _array_index) (`/Game/Blueprints/GameStateVR.TargetLocations` (`self.GameState`))
    (bind _returnvalue (`|SpawnActorFromClass` "/Game/Blueprints/bps/BP_Menu_01.BP_Menu_01_C" (`KismetMathLibrary.MakeTransform` (* (`KismetMathLibrary.Normal` _array_element) 1000.0)) "Undefined" "OverrideRootScale" null _array_index self null))
    (`KismetArrayLibrary.Array_Set` (`self.Menus`) _array_index _returnvalue true))
  (`self.ActivateMenu` true))

(event `GetMenuData`
  (params (Section :type "/Game/Blueprints/enums/EN_MenuSections Enum" :default "NewEnumerator0") (Value :type "Float (double-precision)")))

(event `/Game/Blueprints/BPI_Menu.MenuReport`
  (params (MenuType :type "/Game/Blueprints/enums/EN_MenuSections Enum" :default "NewEnumerator7") (BoxID :type Integer) (CTLeft :type "/Game/Blueprints/enums/EN_ControllerLeft Enum" :default "NewEnumerator0") (CTRight :type "/Game/Blueprints/enums/EN_ControllerRight Enum" :default "NewEnumerator0") (PlayerID :type Integer))
  (`|ExecutionSequence`
    (:`then_0`
      (switch `/Game/Blueprints/enums/EN_ControllerLeft` CTLeft
        (:`NewEnumerator0`
          _)
        (:`NewEnumerator1`
          (goto _label :!via `Reset`))))
    (:`then_1`
      (switch `/Game/Blueprints/enums/EN_ControllerRight` CTRight
        (:`NewEnumerator0`
          _)
        (:`NewEnumerator1`
          (goto _label :!via `Reset`)))))
  (switch `/Game/Blueprints/enums/EN_MenuSections` MenuType
    (:`NewEnumerator0`
      (`/Game/Blueprints/GameStateVR.EnemyPause` (`self.GameState`) false)
      (`self.EnemyPause` false)
      (for _array_element (`self.Menus`)
        (`/Game/Blueprints/bps/BP_Menu_01.ChangeText` _array_element "NewEnumerator0" true "Resume")
        (`/Game/Blueprints/bps/BP_Menu_01.ChangeMenuType` _array_element "NewEnumerator0" "NewEnumerator1")
        (`self.ActivateMenu` false)))
    (:`NewEnumerator1`
      (`/Game/Blueprints/GameStateVR.EnemyPause` (`self.GameState`) false)
      (`self.EnemyPause` false)
      (`self.ActivateMenu` false))
    (:`NewEnumerator5`
      (`KismetSystemLibrary.QuitGame` null "Quit" true)
      (`KismetSystemLibrary.ExecuteConsoleCommand` "Exit" null))
    (:`NewEnumerator3`
      (`/Engine/EditorBlueprintResources/StandardMacros.DoOnce` false :!label _label
        (:`Completed`
          (for _array_element_2 (`self.Menus`)
            (`/Game/Blueprints/bps/BP_Menu_01.ChangeValue` _array_element_2 "NewEnumerator3" 0.0)))))))

(event `ActivateMenu`
  (params (Active :type Boolean))
  (for _array_element (`self.Menus`)
    (if Active
      (bind (_returnvalue_x _returnvalue_y) (`KismetMathLibrary.BreakVector` (`self.K2_GetActorLocation` _array_element)))
      (`self.K2_SetActorLocation` _array_element (`KismetMathLibrary.MakeVector` _returnvalue_x _returnvalue_y 160.0) false false)
      (else
        (bind (_returnvalue_x_2 _returnvalue_y_2) (`KismetMathLibrary.BreakVector` (`self.K2_GetActorLocation` _array_element)))
        (`self.K2_SetActorLocation` _array_element (`KismetMathLibrary.MakeVector` _returnvalue_x_2 _returnvalue_y_2 -500.0) false false)))))

(fn `MenuValues`
  (returns (MenuType :type "/Game/Blueprints/enums/EN_MenuSections Enum") (ID :type Integer))
  (return "NewEnumerator7" 0))

(fn `UserConstructionScript`)