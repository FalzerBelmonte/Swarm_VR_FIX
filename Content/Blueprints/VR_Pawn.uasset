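; VR player pawn for a two-controller shooter with an in-game menu, plus first-person movement outside the intro map.
; On introMap it reports ready to GameStateVR, and SetupPlayer spawns a BP_BulletDirector that receives controller button states.
; Tick line-traces from each held trigger hand to feed aim points to the director, or while paused sends controller states to BPI_Menu actors.
; The B buttons toggle the menu and enemy pause through GameState and HUD.
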(event `SetupPlayer`
  (params (ID :type Integer))
  (bind _bulletdamage (`self.BulletDamage`))
  (bind _id (`self.ID`))
  (if (== ID _id)
    (bind _returnvalue (`|SpawnActorFromClass` "/Game/Blueprints/BP_BulletDirector.BP_BulletDirector_C" (`KismetMathLibrary.MakeTransform` (`KismetMathLibrary.MakeVector` (`KismetMathLibrary.Conv_IntToDouble` (* (mod _id 9) 100)) 200.0 200.0)) "Undefined" "OverrideRootScale" null 5.6 false 10000.0 null))
    (bind _output_get (set `self.BulletDirector` _returnvalue))
    (set `/Game/Blueprints/BP_BulletDirector.SpawnerLocation` (`/Game/Blueprints/GameStateVR.SpawnerLocation` (`self.GameState`)) _output_get)
    (set `/Game/Blueprints/BP_BulletDirector.BulletDamage` _bulletdamage _output_get)
    (set `/Game/Blueprints/BP_DataLink.BulletDamage` _bulletdamage (`self.DataLink`))
    (add `/Game/Blueprints/HUD_VR.EnemyPause` (`self.HUD`) (delegate `EnemyPause`))
    (`KismetSystemLibrary.Delay` 0.2)
    (set `self.Active` true)))

(event `EnemyPause`
  (params (Pause :type Boolean))
  (bind _output_get (set `self.MenuActive` Pause))
  (set `/Game/Blueprints/BP_BulletDirector.inMenu` _output_get (stale `SetupPlayer` _output_get)))

(event `self.ReceiveBeginPlay`
  (bind _returnvalue (`GameplayStatics.GetCurrentLevelName` true))
  (if (`KismetStringLibrary.EqualEqual_StrStr` _returnvalue "introMap")
    (set `self.ID` (`PlayerState.PlayerId` (`self.PlayerState`)))
    (bind _ashud_vr (cast `/Game/Blueprints/HUD_VR` (`PlayerController.GetHUD` (`GameplayStatics.GetPlayerController` 0))))
    (set `self.HUD` _ashud_vr)
    (bind _asgame_state_vr (cast `/Game/Blueprints/GameStateVR` (`GameplayStatics.GetGameState`))
      (:`then`
        (bind _output_get (set `self.GameState` _asgame_state_vr))
        (`/Game/Blueprints/GameStateVR.PlayerReady` _output_get (`self.ID`)))
      (:`CastFailed`
        (`KismetSystemLibrary.PrintString` ">>> GameState missing" true true (struct :`R` 0.994792 :`G` 1.0 :`B` 0.989583 :`A` 1.0) 80.0)))
    (else
      (set `self.FirstPersonActive` true)
      (set `self.bUseControllerRotationRoll` true)
      (set `self.bUseControllerRotationPitch` true)
      (set `self.bUseControllerRotationYaw` true))))

(event `InputAxis|MoveForward`
  (params (AxisValue :type "Float (single-precision)"))
  (if (`self.FirstPersonActive`)
    (`self.AddMovementInput` (`KismetMathLibrary.GetForwardVector` (`self.GetControlRotation`)) AxisValue)))

(event `InputAction|Left_A`
  (params (Key :type "Key Structure"))
  (bind _bulletdirector (`self.BulletDirector`))
  (:`Pressed`
    (bind _output_get (set `self.Cntr_L` "NewEnumerator0"))
    (set `/Game/Blueprints/BP_BulletDirector.CNTLeft` _output_get _bulletdirector)
    (if (`self.Active`) :!label _label
      _))
  (:`Released`
    (bind _output_get_2 (set `self.Cntr_L` "NewEnumerator1"))
    (set `/Game/Blueprints/BP_BulletDirector.CNTLeft` _output_get_2 _bulletdirector)
    (goto _label)))

(event `InputAxis|MoveRight`
  (params (AxisValue :type "Float (single-precision)"))
  (if (`self.FirstPersonActive`)
    (`self.AddMovementInput` (`KismetMathLibrary.GetRightVector` (`self.GetControlRotation`)) AxisValue)))

(event `InputAction|Left_B`
  (params (Key :type "Key Structure"))
  (bind _bulletdirector (`self.BulletDirector`))
  (:`Pressed`
    (bind _output_get (set `self.MenuActive` (not (`self.MenuActive`))))
    (bind _output_get_2 (set `/Game/Blueprints/BP_BulletDirector.inMenu` _output_get (`self.BulletDirector`)))
    (`/Game/Blueprints/GameStateVR.EnemyPause` (`self.GameState`) _output_get_2)
    (`/Game/Blueprints/HUD_VR.ActivateMenu` (`self.HUD`) _output_get_2)
    (bind _output_get_3 (set `self.Cntr_L` "NewEnumerator2"))
    (set `/Game/Blueprints/BP_BulletDirector.CNTLeft` _output_get_3 _bulletdirector)
    (goto _label))
  (:`Released`
    (bind _output_get_4 (set `self.Cntr_L` "NewEnumerator3"))
    (set `/Game/Blueprints/BP_BulletDirector.CNTLeft` _output_get_4 _bulletdirector)
    (goto _label)))

(event `InputAxis|Turn`
  (params (AxisValue :type "Float (single-precision)"))
  (if (`self.FirstPersonActive`)
    (`self.AddControllerYawInput` AxisValue)))

(event `InputAction|Left_C`
  (params (Key :type "Key Structure"))
  (bind _bulletdirector (`self.BulletDirector`))
  (:`Pressed`
    (bind _output_get (set `self.Cntr_L` "NewEnumerator4"))
    (set `/Game/Blueprints/BP_BulletDirector.CNTLeft` _output_get _bulletdirector)
    (goto _label))
  (:`Released`
    (bind _output_get_2 (set `self.Cntr_L` "NewEnumerator5"))
    (set `/Game/Blueprints/BP_BulletDirector.CNTLeft` _output_get_2 _bulletdirector)
    (goto _label)))

(event `InputAxis|LookUp`
  (params (AxisValue :type "Float (single-precision)"))
  (if (`self.FirstPersonActive`)
    (`self.AddControllerPitchInput` AxisValue)))

(event `self.ReceiveTick`
  (params (DeltaSeconds :type "Float (single-precision)"))
  (bind _shootr (`self.ShootR`))
  (bind _shootl (`self.ShootL`))
  (bind _shootr_2 (`self.ShootR`))
  (bind _bulletdirector (`self.BulletDirector`))
  (bind _shootl_2 (`self.ShootL`))
  (if (`self.Active`)
    (if (not (`self.MenuActive`))
      (`|ExecutionSequence`
        (:`then_0`
          (switch `/Game/Blueprints/enums/EN_ControllerLeft` (`self.Cntr_L`)
            (:`NewEnumerator0`
              (bind _enemylocation (`self.CheckImpact` (`SceneComponent.K2_GetComponentLocation` _shootl_2) (`SceneComponent.GetForwardVector` _shootl_2) DeltaSeconds))
              (set `/Game/Blueprints/BP_BulletDirector.EnemyLeft` _enemylocation _bulletdirector))))
        (:`then_1`
          (switch `/Game/Blueprints/enums/EN_ControllerRight` (`self.Cntr_R`)
            (:`NewEnumerator0`
              (bind _enemylocation_2 (`self.CheckImpact` (`SceneComponent.K2_GetComponentLocation` _shootr) (`SceneComponent.GetForwardVector` _shootr) DeltaSeconds))
              (set `/Game/Blueprints/BP_BulletDirector.EnemyRight` _enemylocation_2 _bulletdirector)))))
      (set `/Game/Blueprints/BP_BulletDirector.Left` (`SceneComponent.K2_GetComponentLocation` (`self.WPL`)) _bulletdirector)
      (set `/Game/Blueprints/BP_BulletDirector.Right` (`SceneComponent.K2_GetComponentLocation` (`self.WPR`)) _bulletdirector)
      (else
        (`self.CheckMenu` (`SceneComponent.K2_GetComponentLocation` _shootl) (`SceneComponent.GetForwardVector` _shootl) DeltaSeconds)
        (`self.CheckMenu` (`SceneComponent.K2_GetComponentLocation` _shootr_2) (`SceneComponent.GetForwardVector` _shootr_2) DeltaSeconds)))))

(event `InputAction|Right_A`
  (params (Key :type "Key Structure"))
  (bind _bulletdirector (`self.BulletDirector`))
  (:`Pressed`
    (bind _output_get (set `self.Cntr_R` "NewEnumerator0"))
    (set `/Game/Blueprints/BP_BulletDirector.CNTRight` _output_get _bulletdirector)
    (goto _label))
  (:`Released`
    (bind _output_get_2 (set `self.Cntr_R` "NewEnumerator1"))
    (set `/Game/Blueprints/BP_BulletDirector.CNTRight` _output_get_2 _bulletdirector)
    (goto _label)))

(event `InputAction|Right_B`
  (params (Key :type "Key Structure"))
  (bind _bulletdirector (`self.BulletDirector`))
  (:`Pressed`
    (bind _output_get (set `self.MenuActive` (not (`self.MenuActive`))))
    (bind _output_get_2 (set `/Game/Blueprints/BP_BulletDirector.inMenu` _output_get (`self.BulletDirector`)))
    (`/Game/Blueprints/GameStateVR.EnemyPause` (`self.GameState`) _output_get_2)
    (`/Game/Blueprints/HUD_VR.ActivateMenu` (`self.HUD`) _output_get_2)
    (bind _output_get_3 (set `self.Cntr_R` "NewEnumerator2"))
    (set `/Game/Blueprints/BP_BulletDirector.CNTRight` _output_get_3 _bulletdirector)
    (goto _label))
  (:`Released`
    (bind _output_get_4 (set `self.Cntr_R` "NewEnumerator3"))
    (set `/Game/Blueprints/BP_BulletDirector.CNTRight` _output_get_4 _bulletdirector)
    (goto _label)))

(event `InputAction|Right_C`
  (params (Key :type "Key Structure"))
  (bind _bulletdirector (`self.BulletDirector`))
  (:`Pressed`
    (bind _output_get (set `self.Cntr_R` "NewEnumerator4"))
    (set `/Game/Blueprints/BP_BulletDirector.CNTRight` _output_get _bulletdirector)
    (goto _label))
  (:`Released`
    (bind _output_get_2 (set `self.Cntr_R` "NewEnumerator5"))
    (set `/Game/Blueprints/BP_BulletDirector.CNTRight` _output_get_2 _bulletdirector)
    (goto _label)))

(event `GameEnd`
  (`KismetSystemLibrary.QuitGame` null "Quit" true)
  (`KismetSystemLibrary.ExecuteConsoleCommand` "Exit" null))

(fn `CheckImpact`
  (params (Location :type "Vector Structure") (Forward :type "Vector Structure") (DS :type "Float (double-precision)"))
  (returns (EnemyLocation :type "Vector Structure"))
  (bind _returnvalue (+ Location (* Forward (`self.BulletMaxRange`))))
  (bind (_outhit _returnvalue_2) (`KismetSystemLibrary.LineTraceSingleForObjects` :`Start` Location :`End` _returnvalue :`ObjectTypes` (`self.ObjectTypes`) :`DrawDebugType` "ForDuration" :`DrawTime` (* 2 DS)))
  (if _returnvalue_2
    (`|ExecutionSequence`
      (:`then_0`
        (bind (_bblockinghit _binitialoverlap _time _distance _location _impactpoint _normal) (`GameplayStatics.BreakHitResult` _outhit))
        (bind _projectedlocation (`NavigationSystemV1.K2_ProjectPointToNavigation` _location))
        (`KismetSystemLibrary.DrawDebugCylinder` _projectedlocation (+ _projectedlocation (* _normal 4.2))))
      (:`then_1`
        (return _impactpoint)))
    (else
      (return _returnvalue))))

(fn `CheckMenu`
  (params (Location :type "Vector Structure") (Forward :type "Vector Structure") (DS :type "Float (double-precision)"))
  (bind (_outhit _returnvalue) (`KismetSystemLibrary.LineTraceSingleForObjects` :`Start` Location :`End` (+ Location (* Forward (`self.BulletMaxRange`))) :`ObjectTypes` (`self.ObjectTypes`) :`DrawDebugType` "ForDuration" :`TraceColor` (struct :`R` 0.260417 :`G` 0.687573 :`B` 1.0 :`A` 1.0) :`TraceHitColor` (struct :`R` 0.070988 :`G` 0.075674 :`B` 1.0 :`A` 1.0) :`DrawTime` (* 2 DS)))
  (if _returnvalue
    (bind (_bblockinghit _binitialoverlap _time _distance _location _impactpoint _normal _impactnormal _physmat _hitactor) (`GameplayStatics.BreakHitResult` _outhit))
    (if (`KismetSystemLibrary.DoesImplementInterface` _hitactor "/Game/Blueprints/BPI_Menu.BPI_Menu_C")
      (message `/Game/Blueprints/BPI_Menu.MenuController` _hitactor (`self.Cntr_L`) (`self.Cntr_R`) (`PlayerState.PlayerId` (`self.PlayerState`)))
      (bind _projectedlocation (`NavigationSystemV1.K2_ProjectPointToNavigation` _location))
      (`KismetSystemLibrary.DrawDebugCylinder` _projectedlocation (+ _projectedlocation (* _normal 4.2)))
      (return)
      (else
        (return)))
    (else
      (return))))

(fn `UserConstructionScript`)