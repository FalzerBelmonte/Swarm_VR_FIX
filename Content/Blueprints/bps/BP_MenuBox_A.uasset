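; BP_MenuBox_A is a menu box actor with main and side text, identified by a MenuType and ID.
; MenuController plays a timeline in reverse to tint the box's dynamic material, and its updates report the input and player to the owner through BPI_Menu after a short delay.
; Events change the type and text or toggle Easy/Hard.
; Older click and value-stepping logic is left disconnected.
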(event `self.ReceiveBeginPlay`
  (bind _menutype (`self.MenuType`))
  (`SceneComponent.SetVisibility` (`self.Cube4`) true true)
  (`self.SetMainBoxText` _menutype (`self.infoMain`))
  (`self.SetSideBoxText` _menutype (`self.infoSide`))
  (bind _returnvalue (`PrimitiveComponent.CreateDynamicMaterialInstance` (`self.Cube5`) 0 "/Game/Mats/MTS_03_A.MTS_03_A" "None"))
  (set `self.Mat_01` _returnvalue))

(event `self.ReceiveTick`
  (params (DeltaSeconds :type "Float (single-precision)")))

(event `/Game/Blueprints/BPI_Menu.MenuController`
  (params (CTLeft :type "/Game/Blueprints/enums/EN_ControllerLeft Enum" :default "NewEnumerator0") (CTRight :type "/Game/Blueprints/enums/EN_ControllerRight Enum" :default "NewEnumerator0") (PlayerID :type Integer))
  (bind _returnvalue (`self.GetOwner`))
  (bind (_direction _t01) (`Timeline|Timeline_0` :!via `ReverseFromEnd`)
    (:`Update`
      (`MaterialInstanceDynamic.SetVectorParameterValue` (`self.Mat_01`) "Color" _t01)
      (if (`KismetSystemLibrary.DoesImplementInterface` _returnvalue "/Game/Blueprints/BPI_Menu.BPI_Menu_C")
        (`KismetSystemLibrary.Delay` (* 6 (`GameplayStatics.GetWorldDeltaSeconds`)))
        (message `/Game/Blueprints/BPI_Menu.MenuReport` _returnvalue (`self.MenuType`) (`self.ID`) CTLeft CTRight PlayerID)))))

(event `SetMenuType`
  (params (MenyType :type "/Game/Blueprints/enums/EN_MenuSections Enum" :default "NewEnumerator7") (NewMenuType :type "/Game/Blueprints/enums/EN_MenuSections Enum" :default "NewEnumerator7"))
  (if (== (`self.MenuType`) MenyType)
    (set `self.MenuType` NewMenuType)))

(event `SetValue`
  (params (Section :type "/Game/Blueprints/enums/EN_MenuSections Enum" :default "NewEnumerator0") (Value :type "Float (double-precision)"))
  (if (`|EnumEquality` Section "NewEnumerator3")
    (if (`KismetStringLibrary.EqualEqual_StrStr` (`self.infoMain`) "Easy")
      (set `self.infoMain` "Hard")
      (else
        (set `self.infoMain` "Easy")))
    (`self.SetMainBoxText` "NewEnumerator3" (`self.infoMain`))))

(event `SetMainBoxText`
  (params (MenuType :type "/Game/Blueprints/enums/EN_MenuSections Enum" :default "NewEnumerator7") (info :type String))
  (if (== (`self.MenuType`) MenuType)
    (`TextRenderComponent.K2_SetText` (`self.MBText`) (`KismetTextLibrary.Conv_StringToText` info))))

(event `SetSideBoxText`
  (params (ManuType :type "/Game/Blueprints/enums/EN_MenuSections Enum" :default "NewEnumerator7") (info :type String))
  (if (== (`self.MenuType`) ManuType)
    (`TextRenderComponent.K2_SetText` (`self.SBText`) (`KismetTextLibrary.Conv_StringToText` info))))

(fn `MenuValues`
  (returns (MenuType :type "/Game/Blueprints/enums/EN_MenuSections Enum") (ID :type Integer))
  (return (`self.MenuType`) (`self.ID`)))

(fn `UserConstructionScript`)