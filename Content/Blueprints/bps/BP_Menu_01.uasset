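; Main menu actor that shows Start Game, Difficulty and Exit Game boxes on three billboard anchors.
; Shortly after BeginPlay it rotates toward the world origin, then spawns the BP_MenuBox_A actors, owned by the HUD, and attaches them.
; MenuReport forwards box reports to the HUD.
; ChangeText, ChangeMenuType and ChangeValue update whichever boxes match the given menu type.
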(event `self.ReceiveBeginPlay`
  (`KismetSystemLibrary.Delay` 0.2)
  (`self.K2_SetActorRotation` (`KismetMathLibrary.FindLookAtRotation` (`self.K2_GetActorLocation`) (0.0 0.0 0.0)))
  (`self.AddMenuBox`))

(event `/Game/Blueprints/BPI_Menu.MenuReport`
  (params (MenuType :type "/Game/Blueprints/enums/EN_MenuSections Enum" :default "NewEnumerator7") (BoxID :type Integer) (CTLeft :type "/Game/Blueprints/enums/EN_ControllerLeft Enum" :default "NewEnumerator0") (CTRight :type "/Game/Blueprints/enums/EN_ControllerRight Enum" :default "NewEnumerator0") (PlayerID :type Integer))
  (message `/Game/Blueprints/BPI_Menu.MenuReport` (`self.HUD`) MenuType BoxID CTLeft CTRight PlayerID)
  (if (or (`|EnumEquality` CTLeft "NewEnumerator0") (`|EnumEquality` CTRight "NewEnumerator0"))
    (switch `/Game/Blueprints/enums/EN_MenuSections` "NewEnumerator0")))

(event `ChangeText`
  (params (MenuType :type "/Game/Blueprints/enums/EN_MenuSections Enum" :default "NewEnumerator7") (MainBox :type Boolean) (info :type String))
  (for _array_element (`self.MenuBox`)
    (if (== (`/Game/Blueprints/bps/BP_MenuBox_A.MenuType` _array_element) MenuType)
      (if MainBox
        (`/Game/Blueprints/bps/BP_MenuBox_A.SetMainBoxText` _array_element MenuType info)
        (else
          (`/Game/Blueprints/bps/BP_MenuBox_A.SetSideBoxText` _array_element MenuType info))))))

(event `ChangeMenuType`
  (params (Current :type "/Game/Blueprints/enums/EN_MenuSections Enum" :default "NewEnumerator7") (New :type "/Game/Blueprints/enums/EN_MenuSections Enum" :default "NewEnumerator7"))
  (for _array_element (`self.MenuBox`)
    (if (== (`/Game/Blueprints/bps/BP_MenuBox_A.MenuType` _array_element) Current)
      (`/Game/Blueprints/bps/BP_MenuBox_A.SetMenuType` _array_element Current New))))

(event `ChangeValue`
  (params (MenuType :type "/Game/Blueprints/enums/EN_MenuSections Enum" :default "NewEnumerator7") (Value :type "Float (double-precision)"))
  (for _array_element (`self.MenuBox`)
    (if (== (`/Game/Blueprints/bps/BP_MenuBox_A.MenuType` _array_element) MenuType)
      (`/Game/Blueprints/bps/BP_MenuBox_A.SetValue` _array_element MenuType Value))))

(fn `AddMenuBox`
  (`|ExecutionSequence`
    (:`then_0`
      (bind _returnvalue (`|SpawnActorFromClass` "/Game/Blueprints/bps/BP_MenuBox_A.BP_MenuBox_A_C" (`KismetMathLibrary.MakeTransform` (0.0 0.0 0.0)) "Undefined" "OverrideRootScale" null true 0 "Start Game" "" 0.0 "NewEnumerator0" 1.0 20.0 null))
      (`self.SetOwner` _returnvalue (`self.HUD`))
      (`KismetArrayLibrary.Array_Set` (`self.MenuBox`) 0 _returnvalue true)
      (`self.K2_AttachToComponent` _returnvalue (`|GetArrayItem` (`self.MenuLocations`)) "None" "KeepRelative" "KeepRelative" "KeepRelative" true))
    (:`then_1`
      (bind _returnvalue_2 (`|SpawnActorFromClass` "/Game/Blueprints/bps/BP_MenuBox_A.BP_MenuBox_A_C" (`KismetMathLibrary.MakeTransform` (0.0 0.0 0.0)) "Undefined" "OverrideRootScale" null true 1 "Easy" "Difficulty" 0.0 "NewEnumerator3" 1.0 20.0 null))
      (`self.SetOwner` _returnvalue_2 (`self.HUD`))
      (`KismetArrayLibrary.Array_Set` (`self.MenuBox`) 1 _returnvalue_2 true)
      (`self.K2_AttachToComponent` _returnvalue_2 (`|GetArrayItem` (`self.MenuLocations`) 1) "None" "KeepRelative" "KeepRelative" "KeepRelative" true))
    (:`then_2`
      (bind _returnvalue_3 (`|SpawnActorFromClass` "/Game/Blueprints/bps/BP_MenuBox_A.BP_MenuBox_A_C" (`KismetMathLibrary.MakeTransform` (0.0 0.0 0.0)) "Undefined" "OverrideRootScale" null true 2 "Exit Game" "" 0.0 "NewEnumerator5" 1.0 20.0 null))
      (`self.SetOwner` _returnvalue_3 (`self.HUD`))
      (`KismetArrayLibrary.Array_Set` (`self.MenuBox`) 2 _returnvalue_3 true)
      (`self.K2_AttachToComponent` _returnvalue_3 (`|GetArrayItem` (`self.MenuLocations`) 2) "None" "KeepRelative" "KeepRelative" "KeepRelative" true))
    (:`then_3`
      (return))))

(fn `MenuValues`
  (returns (MenuType :type "/Game/Blueprints/enums/EN_MenuSections Enum") (ID :type Integer))
  (return "NewEnumerator7" 0))

(fn `UserConstructionScript`
  (bind _menulocations (`self.MenuLocations`))
  (`KismetArrayLibrary.Array_Set` _menulocations 0 (`self.Billboard1`) true)
  (`KismetArrayLibrary.Array_Set` _menulocations 1 (`self.Billboard2`) true)
  (`KismetArrayLibrary.Array_Set` _menulocations 2 (`self.Billboard3`) true))