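; BP_SPL_01 is a spline path spawner that creates a population of BP_SwarmAI_03 swarms when play begins.
; The construction script sorts its spline components into main and alternate sets, using "Alternate" in the component name.
; Each swarm spawns at the actor's location, facing a random spline from the set chosen by PathDefault.
; It receives quantity, speed and index on spawn, then that spline through EnemyBegin.
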(event `self.ReceiveBeginPlay`
  (bind _splines_02 (`self.Splines_02`))
  (bind _splines_01 (`self.Splines_01`))
  (for _index (range (`self.Population`))
    (if (`self.PathDefault`)
      (set `self.temp_Spline` (`|GetArrayItem` _splines_01 (`KismetMathLibrary.RandomIntegerInRange` 0 (- (`KismetArrayLibrary.Array_Length` _splines_01) 1))))
      (else
        (set `self.temp_Spline` (`|GetArrayItem` _splines_02 (`KismetMathLibrary.RandomIntegerInRange` 0 (- (`KismetArrayLibrary.Array_Length` _splines_02) 1))))))
    (bind _returnvalue (`|SpawnActorFromClass` "/Game/Blueprints/bps/BP_SwarmAI_03.BP_SwarmAI_03_C" (`KismetMathLibrary.MakeTransform` (`self.K2_GetActorLocation`) (`SceneComponent.K2_GetComponentRotation` (`self.temp_Spline`))) "AlwaysSpawn" "OverrideRootScale" null (`self.Quantity`) null 500.0 1000.0 (`self.MoveSpeed`) _index null))
    (`/Game/Blueprints/bps/BP_SwarmAI_03.EnemyBegin` _returnvalue (`self.temp_Spline`))))

(fn `UserConstructionScript`
  (`KismetArrayLibrary.Array_Clear` (`self.Splines_01`))
  (`KismetArrayLibrary.Array_Clear` (`self.Splines_02`))
  (set `self.Main Spline Path Count` 0)
  (set `self.Alternate Spline Path Count` 0)
  (for _array_element (`self.K2_GetComponentsByClass` "/Script/Engine.SplineComponent")
    (if (`KismetStringLibrary.Contains` (`KismetSystemLibrary.GetDisplayName` _array_element) "Alternate")
      (`KismetArrayLibrary.Array_Add` (`self.Splines_02`) _array_element)
      (else
        (`KismetArrayLibrary.Array_Add` (`self.Splines_01`) _array_element)))))