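; BP_ScoreBoard is a scoreboard actor that keeps a running integer score and displays it on a text render component.
; ReportTypeA compares the incoming ID with the board's own, adds the truncated incoming value on a match and refreshes the text.
; ReportValue exposes the total as a float with the ID, while ReportController returns default enum values for both hands.
; BeginPlay caches GameStateVR, which the shown graphs never use.
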(event `/Game/Blueprints/BPI_Report.ReportTypeA`
  (params (Value :type "Float (single-precision)") (ID :type Integer))
  (if (== ID (`self.ID`))
    (bind _output_get (set `self.Value` (+ (`KismetMathLibrary.FTrunc` Value) (`self.Value`))))
    (`TextRenderComponent.K2_SetText` (`self.TextRender`) (`KismetTextLibrary.Conv_IntToText` _output_get))))

(event `self.ReceiveBeginPlay`
  (bind _asgame_state_vr (cast `/Game/Blueprints/GameStateVR` (`GameplayStatics.GetGameState`)))
  (set `self.GameState` _asgame_state_vr))

(fn `ReportController`
  (returns (Left :type "/Game/Blueprints/enums/EN_ControllerLeft Enum") (Right :type "/Game/Blueprints/enums/EN_ControllerRight Enum"))
  (return "NewEnumerator0" "NewEnumerator0"))

(fn `ReportValue`
  (returns (Value :type "Float (double-precision)") (ID :type Integer))
  (return (`KismetMathLibrary.Conv_IntToDouble` (`self.Value`)) (`self.ID`)))

(fn `UserConstructionScript`)